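; Campfire interactable actor that lets the player heal, spawning enemies each time it is used.
; Box collider overlaps show or hide the interaction widget and enable or disable the actor's input, without checking which actor overlaps.
; Pressing Interact calls HealSelf on the BP_Knight reference cached at BeginPlay, then spawns a BP_Enemy at every SpawnPoint location.
; BeginPlay also creates a WP_Campfire widget that is never used.
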(event OnComponentBeginOverlap(BoxCollider)
  (params (OverlappedComponent :type Primitive%20Component%20Object%20Reference) (OtherActor :type Actor%20Object%20Reference) (OtherComp :type Primitive%20Component%20Object%20Reference) (OtherBodyIndex :type Integer) (bFromSweep :type Boolean) (SweepResult :type Hit%20Result%20Structure%20%28by%20ref%29))
  ;[1 1 1] Within Campfire range, display interaction text
  (Development|PrintString "Entered campfire collision range")
  (Widget|SetVisibility (UserInterface|GetUserWidgetObject (Variables|Default|GetInteraction%20Widget)) "Visible")
  (Input|EnableInput (Game|GetPlayerController 0)))

(event OnComponentEndOverlap(BoxCollider)
  (params (OverlappedComponent :type Primitive%20Component%20Object%20Reference) (OtherActor :type Actor%20Object%20Reference) (OtherComp :type Primitive%20Component%20Object%20Reference) (OtherBodyIndex :type Integer))
  ;[1 1 1] Within Campfire range, display interaction text
  (Development|PrintString "Exited campfire collision range")
  (Widget|SetVisibility (UserInterface|GetUserWidgetObject (Variables|Default|GetInteraction%20Widget)) "Hidden")
  (Input|DisableInput (Game|GetPlayerController 0)))

(event EventBeginPlay
  ;[1 1 1] Create Interaction text widget
  (Utilities|FlowControl|Sequence
    (:then_0
      ;[1 1 1] Reference to Player in world
      (bind _asbp_knight (Utilities|Casting|CastToBP_Knight (Game|GetPlayerCharacter 0)))
      (Variables|Default|SetPlayer _asbp_knight))
    (:then_1
      (UserInterface|CreateWidget "/Game/UserInterface/Campfire/WP_Campfire.WP_Campfire_C"))))

(event Collision|EventActorBeginOverlap
  (params (OtherActor :type Actor%20Object%20Reference)))

(event EventTick
  (params (DeltaSeconds :type Float%20%28single-precision%29)))

(event Input|ActionEvents|InputActionInteract
  (params (Key :type Key%20Structure))
  ;[1 1 1] When input is enabled, allow to call HealSelf
  (:Pressed
    (Default|HealSelf (Variables|Default|GetPlayer))
    ;[1 1 1] Spawn Enemy
    (for _array_element (Variables|Default|GetSpawnPoint)
      (Game|SpawnActorfromClass "/Game/ThirdPersonCPP/Blueprints/BP_Enemy.BP_Enemy_C" (Math|Conversions|ToTransform(Vector) (Transformation|GetWorldLocation (Variables|/Script/Engine.Actor|GetRootComponent _array_element))) "Undefined" _array_element 0))))

(fn ConstructionScript)