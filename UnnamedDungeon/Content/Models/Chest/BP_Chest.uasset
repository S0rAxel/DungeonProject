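; Openable treasure chest that shows an interaction widget and enables input while a BP_Knight overlaps it and it is still closed.
; Pressing Interact marks it open, swings the lid pivot with a timeline, hides the prompt and disables input.
; After a short delay it spawns BP_Coin actors at the spawn point with random rotations, driven by CoinsInChest.
; Tick turns the widget toward the camera horizontally, then adds a fixed local rotation offset.
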(event Collision|EventActorBeginOverlap
  (params (OtherActor :type Actor%20Object%20Reference))
  (bind _widget (Variables|Default|GetWidget))
  (bind _returnvalue (UserInterface|GetUserWidgetObject _widget))
  ;[1 1 1] Set Visibility for Widget
  (bind _asbp_knight (Utilities|Casting|CastToBP_Knight OtherActor))
  (Utilities|IsValid _asbp_knight
    (:Is%20Valid
      (if (not (Variables|Default|GetisOpen))
        (Utilities|IsValid _returnvalue
          (:Is%20Valid
            (Widget|SetVisibility _returnvalue "Visible")
            (Input|EnableInput (Game|GetPlayerController 0))))))))

(event EventTick
  (params (DeltaSeconds :type Float%20%28single-precision%29))
  (bind _widget (Variables|Default|GetWidget))
  ;[1 1 1] Widget looking at the camera
  (Utilities|IsValid (Variables|Default|GetWidget)
    (:Is%20Valid
      (Transformation|SetWorldRotation _widget (Math|Conversions|RotationFromXVector (Math|Vector|RotateVector (Class|KismetMathLibrary|VectorNormalUnsafe (* (- (Transformation|GetActorLocation (Game|GetPlayerCameraManager 0)) (Transformation|GetWorldLocation (Variables|Default|GetWidget))) "1.000000,1.000000, 0")) "0, 0, 0")) false false)
      (Transformation|AddLocalRotation _widget "70.000000, 0,0.000000" false false))))

(event EventBeginPlay
  (bind _widget (Variables|Default|GetWidget))
  (bind _returnvalue (UserInterface|GetUserWidgetObject _widget))
  ;[1 1 1] Initialize Widget
  (Utilities|IsValid _returnvalue
    (:Is%20Valid
      (Widget|SetVisibility _returnvalue "Hidden"))))

(event Collision|EventActorEndOverlap
  (params (OtherActor :type Actor%20Object%20Reference))
  (bind _widget (Variables|Default|GetWidget))
  (bind _returnvalue (UserInterface|GetUserWidgetObject _widget))
  ;[1 1 1] Set Visibility for Widget
  (bind _asbp_knight (Utilities|Casting|CastToBP_Knight OtherActor))
  (Utilities|IsValid _asbp_knight
    (:Is%20Valid
      (Utilities|IsValid _returnvalue
        (:Is%20Valid
          (Widget|SetVisibility _returnvalue "Hidden")
          (Input|DisableInput (Game|GetPlayerController 0)))))))

(event Input|ActionEvents|InputActionInteract
  (params (Key :type Key%20Structure))
  (bind _widget (Variables|Default|GetWidget))
  (bind _pivotchest (Variables|Default|GetPivotChest))
  (bind _spawnpoint (Variables|Default|GetSpawnPoint))
  (bind _returnvalue (Transformation|GetWorldRotation _pivotchest))
  (bind _returnvalue_2 (Transformation|GetWorldTransform _spawnpoint))
  (bind _returnvalue_3 (UserInterface|GetUserWidgetObject _widget))
  ;[1 1 1] Interaction
  (:Pressed
    (Variables|Default|SetisOpen true)
    (Utilities|FlowControl|Sequence
      (:then_0
        (bind _dooropening (Timeline|Timeline Play)
          (:Update
            (Transformation|SetWorldRotation _pivotchest (Math|Rotator|MakeRotator (+ (.roll _returnvalue) _dooropening) (.pitch _returnvalue) (.yaw _returnvalue)) false false))))
      (:then_1
        (Utilities|FlowControl|Delay 0.6)
        (for _index (range 0 (Variables|Default|GetcoinsInChest))
          (Game|SpawnActorfromClass "/Game/Models/Coin/BP_Coin.BP_Coin_C" (Math|Transform|MakeTransform (Math|Vector|MakeVector (.x (.location _returnvalue_2)) (.y (.location _returnvalue_2)) (.z (.location _returnvalue_2))) (Math|Random|RandomRotator false) (.scale _returnvalue_2)) "Undefined" 0 0)))
      (:then_2
        (Utilities|IsValid _returnvalue_3
          (:Is%20Valid
            (Widget|SetVisibility _returnvalue_3 "Hidden")
            (Input|DisableInput (Game|GetPlayerController 0))))))))

(fn ConstructionScript)