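; BP_Potion is an interactable health pickup that adds one Health to the BP_Knight player and destroys itself when Interact is pressed.
; Overlap with a BP_Knight shows or hides the interaction widget and enables or disables the potion's input.
; Every tick, the widget turns toward the camera on the horizontal plane with a fixed offset, while the potion spins and bobs on a sine wave, whose per-frame step ignores delta time.
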(event EventBeginPlay
  (bind _interaction_widget (Variables|Default|GetInteraction%20Widget))
  (bind _returnvalue (UserInterface|GetUserWidgetObject _interaction_widget))
  ;[1 1 1] Getting player & Initializing Widger key
  (bind _asbp_knight (Utilities|Casting|CastToBP_Knight (Game|GetPlayerCharacter 0)))
  (Variables|Default|SetPlayer _asbp_knight)
  (Utilities|IsValid _returnvalue
    (:Is%20Valid
      (Widget|SetVisibility _returnvalue "Hidden"))))

(event Collision|EventActorBeginOverlap
  (params (OtherActor :type Actor%20Object%20Reference))
  (bind _interaction_widget (Variables|Default|GetInteraction%20Widget))
  (bind _returnvalue (UserInterface|GetUserWidgetObject _interaction_widget))
  ;[1 1 1] Set Visibility for Widget
  (bind _asbp_knight (Utilities|Casting|CastToBP_Knight OtherActor))
  (Utilities|IsValid _asbp_knight
    (:Is%20Valid
      (Utilities|IsValid _returnvalue
        (:Is%20Valid
          (Widget|SetVisibility _returnvalue "Visible")
          (Input|EnableInput (Game|GetPlayerController 0)))))))

(event EventTick
  (params (DeltaSeconds :type Float%20%28single-precision%29))
  (bind _interaction_widget (Variables|Default|GetInteraction%20Widget))
  (Utilities|FlowControl|Sequence
    (:then_0
      ;[1 1 1] Widget looking at the camera
      (Utilities|IsValid (Variables|Default|GetInteraction%20Widget)
        (:Is%20Valid
          (Transformation|SetWorldRotation _interaction_widget (Math|Conversions|RotationFromXVector (Math|Vector|RotateVector (Class|KismetMathLibrary|VectorNormalUnsafe (* (- (Transformation|GetActorLocation (Game|GetPlayerCameraManager 0)) (Transformation|GetWorldLocation (Variables|Default|GetInteraction%20Widget))) "1.000000,1.000000, 0")) "0, 0,0.000000")) false false)
          (Transformation|AddLocalRotation _interaction_widget "70.000000, 0,0.000000" false false))))
    (:then_1
      ;[1 1 1] Rotation and Hover
      (Transformation|AddLocalRotation (Variables|Default|GetPotion) (Math|Rotator|MakeRotator 0.0 0.0 (* DeltaSeconds 1e+02)) false false)
      (Transformation|AddRelativeLocation (Variables|Default|GetPotion) (Math|Vector|MakeVector 0.0 0.0 (Math|Float|Clamp(Float) (Math|Trig|Sin(Radians) (* (Utilities|Time|GetRealTimeSeconds) 5.0)) -1.0)) false false))))

(event Collision|EventActorEndOverlap
  (params (OtherActor :type Actor%20Object%20Reference))
  (bind _interaction_widget (Variables|Default|GetInteraction%20Widget))
  (bind _returnvalue (UserInterface|GetUserWidgetObject _interaction_widget))
  ;[1 1 1] Set Visibility for Widget
  (bind _asbp_knight (Utilities|Casting|CastToBP_Knight OtherActor))
  (Utilities|IsValid _asbp_knight
    (:Is%20Valid
      (Utilities|IsValid _returnvalue
        (:Is%20Valid
          (Widget|SetVisibility _returnvalue "Hidden")
          (Input|DisableInput (Game|GetPlayerController 0)))))))

(event Input|ActionEvents|InputActionInteract
  (params (Key :type Key%20Structure))
  ;[1 1 1] Interaction
  (:Pressed
    (Math|Float|IncrementFloat (Variables|/Game/ThirdPersonCPP/Blueprints/BP_Knight.BP_Knight_C|GetHealth (Variables|Default|GetPlayer))
      (:%20%20
        (Actor|DestroyActor)))))

(fn ConstructionScript)